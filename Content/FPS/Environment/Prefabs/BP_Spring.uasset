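; BP_Spring is a spring prefab that launches the player when they enter its box trigger.
; On overlap, it launches BP_PlayerCharacter along the Arrow component's forward vector at a fixed speed, adding to current velocity rather than overriding it.
; It also disables CanLaunchCharacters on the player's ParkourMovement while inside the box and re-enables it when the overlap ends.
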(event OnComponentBeginOverlap(Box)
  (params (OverlappedComponent :type Primitive%20Component%20Object%20Reference) (OtherActor :type Actor%20Object%20Reference) (OtherComp :type Primitive%20Component%20Object%20Reference) (OtherBodyIndex :type Integer) (bFromSweep :type Boolean) (SweepResult :type Hit%20Result%20Structure%20%28by%20ref%29))
  (bind _asbp_player_character (Utilities|Casting|CastToBP_PlayerCharacter OtherActor))
  (Variables|/Game/FPS/Blueprints/BlueprintsComponents/AC_Parkour.AC_Parkour_C|SetCanLaunchCharacters (Variables|/Game/FPS/Blueprints/CharacterAndClasses/BP_PlayerCharacter.BP_PlayerCharacter_C|GetParkourMovement _asbp_player_character) false)
  (Character|LaunchCharacter _asbp_player_character (* (Math|Vector|GetForwardVector (Variables|Default|GetArrow)) 1.1e+03) false false))

(event OnComponentEndOverlap(Box)
  (params (OverlappedComponent :type Primitive%20Component%20Object%20Reference) (OtherActor :type Actor%20Object%20Reference) (OtherComp :type Primitive%20Component%20Object%20Reference) (OtherBodyIndex :type Integer))
  (bind _asbp_player_character (Utilities|Casting|CastToBP_PlayerCharacter OtherActor))
  (Variables|/Game/FPS/Blueprints/BlueprintsComponents/AC_Parkour.AC_Parkour_C|SetCanLaunchCharacters (Variables|/Game/FPS/Blueprints/CharacterAndClasses/BP_PlayerCharacter.BP_PlayerCharacter_C|GetParkourMovement _asbp_player_character) true))

(event EventBeginPlay)

(event Collision|EventActorBeginOverlap
  (params (OtherActor :type Actor%20Object%20Reference)))

(event EventTick
  (params (DeltaSeconds :type Float%20%28single-precision%29)))

(fn ConstructionScript)