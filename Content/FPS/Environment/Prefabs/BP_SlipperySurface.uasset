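; BP_SlipperySurface is a placeable trigger volume that makes the player character slide while inside it.
; On box overlap it zeroes ground friction, lowers walking braking deceleration and stops the ParkourMovement component from changing friction.
; Leaving the box re-enables that and has ParkourMovement reset friction.
; The construction script scales the box and plane from a Size variable and toggles the plane's visibility.
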(event OnComponentBeginOverlap(Box)
  (params (OverlappedComponent :type Primitive%20Component%20Object%20Reference) (OtherActor :type Actor%20Object%20Reference) (OtherComp :type Primitive%20Component%20Object%20Reference) (OtherBodyIndex :type Integer) (bFromSweep :type Boolean) (SweepResult :type Hit%20Result%20Structure%20%28by%20ref%29))
  (bind _asbp_player_character (Utilities|Casting|CastToBP_PlayerCharacter OtherActor))
  (Variables|/Script/Engine.CharacterMovementComponent|SetGroundFriction (Variables|/Script/Engine.Character|GetCharacterMovement _asbp_player_character) 0.0)
  (Variables|/Script/Engine.CharacterMovementComponent|SetBrakingDecelerationWalking (Variables|/Script/Engine.Character|GetCharacterMovement _asbp_player_character) 1e+02)
  (Variables|/Game/FPS/Blueprints/BlueprintsComponents/AC_Parkour.AC_Parkour_C|SetCanChangeFirction (Variables|/Game/FPS/Blueprints/CharacterAndClasses/BP_PlayerCharacter.BP_PlayerCharacter_C|GetParkourMovement _asbp_player_character) false))

(event OnComponentEndOverlap(Box)
  (params (OverlappedComponent :type Primitive%20Component%20Object%20Reference) (OtherActor :type Actor%20Object%20Reference) (OtherComp :type Primitive%20Component%20Object%20Reference) (OtherBodyIndex :type Integer))
  (bind _asbp_player_character (Utilities|Casting|CastToBP_PlayerCharacter OtherActor))
  (Variables|/Game/FPS/Blueprints/BlueprintsComponents/AC_Parkour.AC_Parkour_C|SetCanChangeFirction (Variables|/Game/FPS/Blueprints/CharacterAndClasses/BP_PlayerCharacter.BP_PlayerCharacter_C|GetParkourMovement _asbp_player_character) true)
  (Default|ResetFirction (Variables|/Game/FPS/Blueprints/CharacterAndClasses/BP_PlayerCharacter.BP_PlayerCharacter_C|GetParkourMovement _asbp_player_character)))

(fn ConstructionScript
  (bind _size (Variables|Default|GetSize))
  (Rendering|SetVisibility (Variables|Default|GetPlane) (Variables|Default|GetShowPlan?) false)
  (Transformation|SetRelativeScale3D (Variables|Default|GetBox) (Math|Vector|MakeVector _size _size 1.0)))