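; BP_Ruler is an editor measuring tool that displays the length of its spline as text in the level.
; The Construction Script places a TextRender at the spline's midpoint and sets its text to the spline length.
; The label's yaw follows the spline direction at that point plus an adjustable Angle offset, with pitch and roll held at zero.
; The event graph holds no active logic.
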(event EventBeginPlay)

(event Collision|EventActorBeginOverlap
  (params (OtherActor :type Actor%20Object%20Reference)))

(event EventTick
  (params (DeltaSeconds :type Float%20%28single-precision%29)))

(fn ConstructionScript
  (bind _spline (Variables|Default|GetSpline))
  (bind _returnvalue (Spline|GetSplineLength _spline))
  (bind _returnvalue_2 (/ _returnvalue 2.0))
  (Transformation|SetRelativeLocation (Variables|Default|GetTextRender) (Spline|GetLocationatDistanceAlongSpline _spline _returnvalue_2 "Local") false false)
  (Transformation|SetRelativeRotation (Variables|Default|GetTextRender) (Math|Rotator|MakeRotator 0.0 0.0 (+ (.yaw (Spline|GetRotationatDistanceAlongSpline _spline _returnvalue_2 "Local")) (Variables|Default|GetAngle))) false false)
  (Rendering|Components|TextRender|SetText (Variables|Default|GetTextRender) (Utilities|Text|ToText(Float) _returnvalue "HalfToEven")))