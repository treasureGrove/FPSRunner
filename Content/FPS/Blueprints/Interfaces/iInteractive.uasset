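; Blueprint interface for world objects that a pawn can interact with in the FPS game.
; It declares hover begin and end, interaction begin, end and execute events, with the instigating pawn passed to the start and execute calls.
; Query functions expose whether interaction can be attempted, plus a description, icon and interact time, suggesting support for prompts and timed interactions.
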(fn Interact
  (params (InstigatorPawn :type Pawn%20Object%20Reference)))

(fn BeginHover
  (params (InstigatorPawn :type Pawn%20Object%20Reference))
  (return))

(fn EndHover)

(fn BeginInteract
  (params (InstigatorPawn :type Pawn%20Object%20Reference))
  (return))

(fn EndInteract)

(fn TrytoInteract
  (return false))

(fn GetDescription
  (return ""))

(fn GetIcon
  (return 0))

(fn GetInteractTime
  (return 0.0))