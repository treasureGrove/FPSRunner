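; Parkour component that gives a character side wall runs, vertical wall runs, ledge grabs, mantling and jump-offs.
; A looping 60 Hz timer feeds gated update graphs, which jumping, falling, landing and cooldown timers open or close.
; Traces select the parkour mode, driving movement through launches, gravity changes and interpolated mantles, with camera tilt and shakes.
; Sprint, crouch and slide are mostly empty stubs.
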(event Custom|JumpEvent
  (if (Utilities|Enum|Equal(Enum) (Variables|Parkour|GetCurrentParkourMode) "NewEnumerator0")
    (if (not (AI|Components|NavMovement|IsFalling (Variables|Default|GetCharacter%20Movement)))
      (CallFunction|OpenGates)
      (CallFunction|PlayCameraShake "/Game/FPS/Blueprints/CameraShake/CS_JumpLand.CS_JumpLand_C"))
    (else
      (CallFunction|JumpEvents))))

(event Custom|Initialize
  (params (Character :type Character%20Object%20Reference) (camera :type Camera%20Component%20Object%20Reference))
  (bind _output_get (Variables|Default|SetCharacter Character))
  (Variables|Default|SetCamera camera)
  (bind _output_get_2 (Variables|Default|SetCharacter%20Movement (Variables|/Script/Engine.Character|GetCharacterMovement _output_get)))
  (Variables|WallRun|SetDefaultGravity (Variables|/Script/Engine.CharacterMovementComponent|GetGravityScale _output_get_2))
  (Utilities|Time|SetTimerbyEvent (delegate Custom|WallRunUpdateEvent) 0.0167 true))

(event Custom|MovementChanged
  (params (PrevMovementMode :type EMovementMode%20Enum :default "MOVE_None") (NewMovementMode :type EMovementMode%20Enum :default "MOVE_None"))
  (Utilities|IsValid (Variables|Default|GetCharacter%20Movement)
    (:Is%20Valid
      (Variables|Parkour|SetPrev%20Movement%20Mode PrevMovementMode)
      (Variables|Parkour|SetCurrent%20Movement%20Mode NewMovementMode)
      (|OpenGatesNode))))

(event Custom|LandEvent
  (WallRun|WallRunEnd 0.0)
  (CallFunction|VerticalWallRunEnd 0.0)
  (CallFunction|CloseGates)
  (CallFunction|PlayCameraShake "/Game/FPS/Blueprints/CameraShake/CS_JumpLand.CS_JumpLand_C")
  (Variables|Default|SetEnableVerticalWallRun true))

(event Custom|WallRunUpdateEvent
  (Utilities|FlowControl|Sequence
    (:then_0
      (|WallRun))
    (:then_1
      (|VerticalWallRun))
    (:then_2
      (|Mantle))
    (:then_3
      (CallFunction|CameraTick))))

(event Custom|DisableVerticalWallRun
  (Utilities|FlowControl|Delay 1.0)
  (Variables|Default|SetEnableVerticalWallRun false))

(event Custom|CrouchSlideEvent)

(event Custom|PlayCameraShake
  (params (Shake :type Legacy%20Camera%20Shake%20Class%20Reference))
  (if (Variables|Default|GetCameraShake)
    (Camera|PlayWorldCameraShake Shake (Transformation|GetActorLocation (Variables|Default|GetCharacter)) 0.0 1e+02)))

(event Custom|ParkourMovementChanged
  (params (PrevParkourMovementMode :type E_ParkourMovementType%20Enum :default "NewEnumerator0") (NewParkourMovementMode :type E_ParkourMovementType%20Enum :default "NewEnumerator0"))
  (Variables|Parkour|SetPrevParkourMode PrevParkourMovementMode)
  (Variables|Parkour|SetCurrentParkourMode NewParkourMovementMode)
  (CallFunction|ResetMovement))

(event Custom|SprintEvent)

(event EventBeginPlay
  (Variables|Parkour|SetCurrentParkourMode "NewEnumerator0"))

(event EventTick
  (params (DeltaSeconds :type Float%20%28single-precision%29))
  (CallFunction|CameraTick))

(fn WallRunUpdate
  (bind _character_movement (Variables|Default|GetCharacter%20Movement))
  (bind _character (Variables|Default|GetCharacter))
  (bind _returnvalue (Transformation|GetVelocity _character))
  (if (Utilities|CanWallRun)
    (bind _onwall (WallRun|WallRunDetection (Transformation|GetActorLocation (Variables|Default|GetCharacter)) (.Right (Utilities|WallRunEndVectors)) -1.0))
    (if _onwall ; rightWallRun
      (CallFunction|SetParkourMovementMode "NewEnumerator2")
      (if (< (.z _returnvalue) 1.5e+02) :!label _label
        (Variables|/Script/Engine.CharacterMovementComponent|SetGravityScale _character_movement (Math|Interpolation|FInterpTo (Variables|/Script/Engine.CharacterMovementComponent|GetGravityScale (Variables|Default|GetCharacter%20Movement)) (Variables|WallRun|GetWallRunTargetGravity) (Utilities|Time|GetWorldDeltaSeconds) 8e+01))
        (if (< (.z _returnvalue) -1.5e+02)
          (Variables|/Script/Engine.MovementComponent|SetVelocity _character_movement (Math|Vector|MakeVector (.x (Variables|/Script/Engine.MovementComponent|GetVelocity _character_movement)) (.y (Variables|/Script/Engine.MovementComponent|GetVelocity _character_movement)) -1.5e+02))))
      (elif (Utilities|Enum|Equal(Enum) (Variables|Parkour|GetCurrentParkourMode) "NewEnumerator2") ; Nolonger wallrunningright
        (WallRun|WallRunEnd 2.0)
        (else
          (bind _onwall_2 (WallRun|WallRunDetection (Transformation|GetActorLocation (Variables|Default|GetCharacter)) (.Left (Utilities|WallRunEndVectors)) 1.0))
          (if _onwall_2
            (CallFunction|SetParkourMovementMode "NewEnumerator1")
            (goto _label)
            (else
              (WallRun|WallRunEnd 2.0))))))
    (else
      (WallRun|WallRunEnd 2.0))))

(fn WallRunJump
  (bind _wallrunnormal (Variables|WallRun|GetWallRunNormal))
  (bind _wallrunjumpoffforce (Variables|WallRun|GetWallRunJumpOffForce))
  (if (Utilities|WallRunning?)
    (WallRun|WallRunEnd 0.15)
    (Character|LaunchCharacter (Variables|Default|GetCharacter) (Math|Vector|MakeVector (* (.x _wallrunnormal) _wallrunjumpoffforce) (* (.y _wallrunnormal) _wallrunjumpoffforce) (Variables|WallRun|GetWallRunJumpHeight)) false true)))

(fn WallRunDetection
  (params (Start :type Vector) (End :type Vector) (WallRunDirection :type Float%20%28double-precision%29))
  (bind _outhit (Collision|LineTraceByChannel Start End "TraceTypeQuery1" false 0 "ForDuration"))
  (if (.bblockinghit _outhit)
    (Variables|WallRun|SetWallRunNormal (.OutValue (Utilities|IsVaildWallRunVector? (.normal _outhit))))
    (if (and (.ReturnValue (Utilities|IsVaildWallRunVector? (.normal _outhit))) (AI|Components|NavMovement|IsFalling (Variables|/Script/Engine.Character|GetCharacterMovement (Variables|Default|GetCharacter))))
      (Character|LaunchCharacter (Variables|Default|GetCharacter) (* (Math|Vector|CrossProduct (Variables|WallRun|GetWallRunNormal) "0.000000,0.000000,1.000000") (* WallRunDirection (Variables|WallRun|GetWallRunSpeed))) (not (Variables|WallRun|GetWallRunGravity)) true)
      (return true)
      (else
        (return false)))
    (else
      (return false))))

(fn WallRunEnd
  (params (ResetTime :type Float%20%28double-precision%29))
  (if (Utilities|WallRunning?)
    (bind _change (CallFunction|SetParkourMovementMode "NewEnumerator0"))
    (if _change
      (CallFunction|CloseWallRunGate)
      (Utilities|Time|SetTimerbyFunctionName 0 "OpenWallRunGate" ResetTime))))

(fn CameraTick
  (switch Utilities|FlowControl|Switch|SwitchonE_ParkourMovementType (Variables|Parkour|GetCurrentParkourMode)
    (:NewEnumerator0
      (CallFunction|CameraTilt 0.0 :!label _label))
    (:NewEnumerator1
      (CallFunction|CameraTilt 15.0))
    (:NewEnumerator2
      (CallFunction|CameraTilt -15.0 :!label _label_2))
    (:NewEnumerator3
      (goto _label))
    (:NewEnumerator4
      (goto _label))
    (:NewEnumerator5
      (goto _label))
    (:NewEnumerator6
      (goto _label_2))
    (:NewEnumerator7
      (goto _label))))

(fn CameraTilt
  (params (TargetX%28Roll%29 :type Float%20%28double-precision%29))
  (bind _camera (Variables|Default|GetCamera))
  (bind _relativerotation (Variables|/Script/Engine.SceneComponent|GetRelativeRotation _camera))
  (bind (_roll _pitch _yaw) (Math|Rotator|BreakRotator _relativerotation))
  (Transformation|SetRelativeRotation _camera (Math|Interpolation|RInterpTo _relativerotation (Math|Rotator|MakeRotator TargetX%28Roll%29 _pitch _yaw) (Utilities|Time|GetWorldDeltaSeconds) 1e+01) false false))

(fn ResetMovement
  (bind _character_movement (Variables|Default|GetCharacter%20Movement))
  (if (Utilities|Enum|Equal(Enum) (Variables|Parkour|GetCurrentParkourMode) "NewEnumerator0")
    (Variables|/Script/Engine.CharacterMovementComponent|SetGravityScale _character_movement (Variables|WallRun|GetDefaultGravity))
    (Pawn|Components|CharacterMovement|SetMovementMode _character_movement (Utilities|Select :Index (Variables|Parkour|GetPrev%20Movement%20Mode) :MOVE_None "MOVE_Falling" :MOVE_Walking "MOVE_Falling" :MOVE_NavWalking "MOVE_Falling" :MOVE_Falling "MOVE_Falling" :MOVE_Swimming "MOVE_Walking" :MOVE_Flying "MOVE_Walking" :MOVE_Custom "MOVE_Walking") 0)))

(fn SetParkourMovementMode
  (params (NewMode :type E_ParkourMovementType%20Enum :default "NewEnumerator0"))
  (if (Utilities|Enum|Equal(Enum) NewMode (Variables|Parkour|GetCurrentParkourMode))
    (return false)
    (else
      (CallFunction|ParkourMovementChanged (Variables|Parkour|GetCurrentParkourMode) NewMode)
      (return true))))

(fn VerticalWallRunUpdate
  (bind (_eyes _feet) (Utilities|MantleVectors))
  (if (Utilities|CanVerticalWallRun)
    (bind (_outhit _returnvalue) (Collision|CapsuleTraceByChannel _eyes _feet 2e+01 1e+01 "TraceTypeQuery1" false 0 "ForDuration" true "(R=0.283880,G=0.763195,B=1.000000,A=1.000000)"))
    (if _returnvalue
      (Variables|Default|SetMantleTraceDistance (.Distance (Collision|BreakHitResult _outhit)))
      (if (Class|CharacterMovementComponent|IsWalkable (Variables|Default|GetCharacter%20Movement) _outhit)
        (Variables|Default|SetMantlePosition (+ (.ImpactPoint (Collision|BreakHitResult _outhit)) (Math|Vector|MakeVector 0.0 0.0 (Variables|/Script/Engine.CapsuleComponent|GetCapsuleHalfHeight (Variables|/Script/Engine.Character|GetCapsuleComponent (Variables|Default|GetCharacter))))))
        (CallFunction|CloseVerticalWallRunGate)
        (|LedgeGrab)
        (if (Utilities|QuickMantle)
          (CallFunction|OpenMantleCheckGate)
          (else
            (Utilities|Time|SetTimerbyFunctionName 0 "OpenMantleCheckGate" 0.25)))
        (else
          (CallFunction|VerticalWallRunMovement :!label _label)))
      (else
        (goto _label)))
    (else
      (CallFunction|VerticalWallRunEnd 0.35))))

(fn VerticalWallRunEnd
  (params (ResetTime :type Float%20%28double-precision%29))
  (bind _currentparkourmode (Variables|Parkour|GetCurrentParkourMode))
  (if (Math|Boolean|ORBoolean (Utilities|Enum|Equal(Enum) _currentparkourmode "NewEnumerator4") (Utilities|Enum|Equal(Enum) _currentparkourmode "NewEnumerator3") (Utilities|Enum|Equal(Enum) _currentparkourmode "NewEnumerator5"))
    (bind _change (CallFunction|SetParkourMovementMode "NewEnumerator0"))
    (if _change
      (CallFunction|CloseVerticalWallRunGate)
      (CallFunction|CloseMantleGate)
      (Utilities|Time|SetTimerbyFunctionName 0 "OpenVerticalWallRunGate" ResetTime))))

(fn VerticalWallRunMovement
  (bind _feet (Utilities|MantleVectors))
  (bind (_outhit _returnvalue) (Collision|LineTraceByChannel _feet (+ _feet (* (Transformation|GetActorForwardVector (Variables|Default|GetCharacter)) 5e+01)) "TraceTypeQuery1" false 0 "ForDuration" true "(R=1.000000,G=0.000000,B=0.947663,A=1.000000)" "(R=0.990454,G=0.885049,B=1.000000,A=1.000000)"))
  (if (and (> (Utilities|ForwardInput) 0.8) _returnvalue)
    (Variables|Default|SetVerticalWallRunNormal (.ImpactNormal (Collision|BreakHitResult _outhit)))
    (CallFunction|SetParkourMovementMode "NewEnumerator3")
    (Character|LaunchCharacter (Variables|Default|GetCharacter) (Math|Vector|MakeVector (.x (* (Variables|Default|GetVerticalWallRunNormal) -6e+02)) (.y (* (Variables|Default|GetVerticalWallRunNormal) -6e+02)) (Variables|Default|GetVerticalWallRunSpeed)) true true)
    (CallFunction|DisableVerticalWallRun)
    (else
      (CallFunction|VerticalWallRunEnd 0.35))))

(fn MantleMovement
  (Transformation|SetActorLocation (Variables|Default|GetCharacter) (Math|Interpolation|VInterpTo (Transformation|GetActorLocation (Variables|Default|GetCharacter)) (Variables|Default|GetMantlePosition) (Utilities|Time|GetWorldDeltaSeconds) (select (Utilities|QuickMantle) (Variables|Default|GetQuickMantleSpeed) (Variables|Default|GetMantleSpeed))) false false)
  (if (< (Math|Vector|Distance(Vector) (Transformation|GetActorLocation (Variables|Default|GetCharacter)) (Variables|Default|GetMantlePosition)) 1e+01)
    (CallFunction|VerticalWallRunEnd 0.5)))

(fn OpenGates
  (CallFunction|OpenWallRunGate)
  (CallFunction|OpenVerticalWallRunGate))

(fn CloseGates
  (CallFunction|CloseWallRunGate)
  (CallFunction|CloseVerticalWallRunGate))

(fn LedgeGrabJump
  (bind _currentparkourmode (Variables|Parkour|GetCurrentParkourMode))
  (bind _verticalwallrunnormal (Variables|Default|GetVerticalWallRunNormal))
  (bind _ledgegrabjumpoffforce (Variables|Default|GetLedgeGrabJumpOffForce))
  (if (Math|Boolean|ORBoolean (Utilities|Enum|Equal(Enum) _currentparkourmode "NewEnumerator4") (Utilities|Enum|Equal(Enum) _currentparkourmode "NewEnumerator3") (Utilities|Enum|Equal(Enum) _currentparkourmode "NewEnumerator5"))
    (CallFunction|VerticalWallRunEnd 0.35)
    (Character|LaunchCharacter (Variables|Default|GetCharacter) (Math|Vector|MakeVector (* (.x _verticalwallrunnormal) _ledgegrabjumpoffforce) (* (.y _verticalwallrunnormal) _ledgegrabjumpoffforce) (Variables|Default|GetLedgeGrabJumpHeight)) true false)))

(fn JumpEvents
  (WallRun|WallRunJump)
  (CallFunction|LedgeGrabJump))

(fn SprintStart
  (CallFunction|CrouchEnd)
  (CallFunction|SlideEnd)
  (if true
    _))

(fn SprintEnd)

(fn CrouchStart)

(fn CrouchEnd)

(fn SlideStart)

(fn SlideEnd)

(event Custom|CloseWallRunGate
  (Utilities|FlowControl|Gate true) ; enters at Close
)

(event Custom|OpenWallRunGate
  (Utilities|FlowControl|Gate true) ; enters at Open
)

(event Custom|OpenMantleGate
  (Utilities|FlowControl|Gate true) ; enters at Open
)

(event Custom|OpenMantleCheckGate
  (Utilities|FlowControl|Gate true) ; enters at Open
)

(event Custom|CloseMantleCheckGate
  (Utilities|FlowControl|Gate true) ; enters at Close
)

(event Custom|MantleCheck
  (if (Utilities|CanMantle)
    (CallFunction|MantleStart)))

(event Custom|MantleStart
  (bind _change (CallFunction|SetParkourMovementMode "NewEnumerator5"))
  (if _change
    (CallFunction|PlayCameraShake (select (Utilities|QuickMantle) "/Game/FPS/Blueprints/CameraShake/CS_QuickMantle.CS_QuickMantle_C" "/Game/FPS/Blueprints/CameraShake/CS_Mantel.CS_Mantel_C"))
    (CallFunction|CloseMantleCheckGate)
    (CallFunction|OpenMantleGate)))

(event Custom|CloseMantleGate
  (Utilities|FlowControl|Gate true) ; enters at Close
)

(event Custom|CloseVerticalWallRunGate
  (CallFunction|CloseMantleGate)
  (Utilities|FlowControl|Gate true) ; enters at Close
)

(event Custom|OpenVerticalWallRunGate
  (Utilities|FlowControl|Gate true) ; enters at Open
)