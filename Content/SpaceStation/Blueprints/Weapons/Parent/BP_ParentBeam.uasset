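; Parent beam weapon Blueprint that fires a continuous damaging laser while BeamActive is set.
; InitBeam loads range, damage, impact effect and sound from DT_WeaponTypes by weapon name.
; Each active Tick line-traces forward from StartPoint and moves the laser's end to the hit or maximum range.
; Hits place the light and impact VFX and apply damage every frame, unscaled by delta time.
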(event Collision|EventActorBeginOverlap
  (params (OtherActor :type Actor%20Object%20Reference)))

(event EventTick
  (params (DeltaSeconds :type Float%20%28single-precision%29))
  (bind _beammaxdistance (Variables|Default|GetBeamMaxDistance))
  (bind _startpoint (Variables|Default|GetStartPoint))
  (bind _pointlight (Variables|Default|GetPointLight))
  (bind _audio (Variables|Default|GetAudio))
  (bind _returnvalue (Transformation|GetWorldLocation _startpoint))
  (bind _returnvalue_2 (Math|Vector|GetForwardVector _startpoint))
  (bind _returnvalue_3 (* _returnvalue_2 _beammaxdistance))
  (bind _returnvalue_4 (+ _returnvalue _returnvalue_3))
  (if (Variables|Default|GetBeamActive)
    (Components|Activation|SetActive _audio true false)
    (Variables|Default|SetBeamEndPoint _returnvalue_4)
    (bind (_outhit _returnvalue_5) (Collision|LineTraceByChannel _returnvalue _returnvalue_4 "TraceTypeQuery1" true 0 "None"))
    (if _returnvalue_5
      (Variables|Default|SetBeamEndPoint (.Location (Collision|BreakHitResult _outhit)))
      (CallFunction|UpdateLaserBeam (Variables|Default|GetBeamEndPoint))
      (Rendering|SetVisibility _pointlight true false)
      (Transformation|SetWorldLocation _pointlight (Variables|Default|GetBeamEndPoint) false false)
      (Transformation|SetWorldTransform (Variables|Default|GetImpactVFX) (Math|Transform|MakeTransform (Variables|Default|GetBeamEndPoint)) false false)
      (Components|Activation|Activate (Variables|Default|GetImpactVFX) false)
      ;[1 1 1] Apply Damage
      (Game|Damage|ApplyDamage (.HitActor (Collision|BreakHitResult _outhit)) (Variables|Default|GetBeamDamage) 0 self)
      (else
        (Rendering|SetVisibility (Variables|Default|GetPointLight) false false)
        (CallFunction|UpdateLaserBeam (Variables|Default|GetBeamEndPoint))
        (Components|Activation|Deactivate (Variables|Default|GetImpactVFX))))
    (else
      (Components|Activation|SetActive _audio false false))))

(event EventBeginPlay)

(fn ConstructionScript
  (bind _endlocation (Variables|Default|GetEndLocation))
  (bind _relativelocation (Variables|/Script/Engine.SceneComponent|GetRelativeLocation _endlocation))
  (bind (_x _y _z) (Math|Vector|BreakVector _relativelocation))
  (Transformation|SetRelativeLocation _endlocation (Math|Vector|MakeVector _x _y (+ _z (Variables|Default|GetBeamMaxDistance))) false false))

(fn UpdateLaserBeam
  (params (EndLocation :type Vector))
  (Class|ParticleSystemComponent|SetBeamEndPoint (Variables|Default|GetLaser) 0 EndLocation))

(fn InitBeam
  (params (WeaponName :type Name))
  ;[1 1 1] Init Beam
  (Transformation|SetWorldLocationAndRotation (Variables|Default|GetLaser) (Transformation|GetWorldLocation (Variables|Default|GetStartPoint)) "0,90.000000, 0" false false)
  (CallFunction|UpdateLaserBeam (Transformation|GetWorldLocation (Variables|Default|GetStartPoint)))
  (bind _returnvalue (Utilities|GetDataTableRow "/Game/SpaceStation/Blueprints/Weapons/Parent/DT_WeaponTypes.DT_WeaponTypes" WeaponName)
    (:then
      (Variables|Default|SetBeamMaxDistance (.BeamDistance (Utilities|Struct|BreakS_WeaponData _returnvalue)))
      (Variables|Default|SetBeamDamage (.BeamDamage (Utilities|Struct|BreakS_WeaponData _returnvalue)))
      (Class|NiagaraComponent|SetAsset (Variables|Default|GetImpactVFX) (.WeaponActionEffect (Utilities|Struct|BreakS_WeaponData _returnvalue)) true)
      (Audio|Components|Audio|SetSound (Variables|Default|GetAudio) (.WeaponActionSound (Utilities|Struct|BreakS_WeaponData _returnvalue))))))