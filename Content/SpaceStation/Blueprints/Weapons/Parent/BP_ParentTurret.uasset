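; Parent turret that automatically tracks and fires on spacecraft inside its detection sphere.
; Overlaps maintain a target list; a random pick drives gated, frame-delayed loops that rotate platform yaw and clamped cannon pitch, resetting when no target remains.
; Once aligned on an unwrecked ship, it spawns projectiles or attached beams at each barrel using DT_WeaponTypes.
; Shots spend ammo, while a looping timer drains it for beams and removes them when firing becomes invalid.
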(event OnComponentBeginOverlap(OverlapDetection)
  (params (OverlappedComponent :type Primitive%20Component%20Object%20Reference) (OtherActor :type Actor%20Object%20Reference) (OtherComp :type Primitive%20Component%20Object%20Reference) (OtherBodyIndex :type Integer) (bFromSweep :type Boolean) (SweepResult :type Hit%20Result%20Structure%20%28by%20ref%29))
  ;[1 1 1] System Detect Something, Check if that's valid actor type for targeting. If true = Allow Shooting
  (bind _asbp_parent_spacecraft (Utilities|Casting|CastToBP_ParentSpacecraft OtherActor))
  (Utilities|Array|Add (Variables|Turret|GetTargetShipsInRange) _asbp_parent_spacecraft)
  (Utilities|IsValid (Variables|Turret|GetCurrentTarget)
    (:Is%20Not%20Valid
      (CallFunction|FindTarget)
      (Variables|Turret|SetShootingPossible true))))

(event OnComponentEndOverlap(OverlapDetection)
  (params (OverlappedComponent :type Primitive%20Component%20Object%20Reference) (OtherActor :type Actor%20Object%20Reference) (OtherComp :type Primitive%20Component%20Object%20Reference) (OtherBodyIndex :type Integer))
  ;[1 1 1] System Detect Something Left from the Detection Range. If Current Target = Disable Shooting
  (bind _asbp_parent_spacecraft (Utilities|Casting|CastToBP_ParentSpacecraft OtherActor))
  (if (Utilities|Array|ContainsItem (Variables|Turret|GetTargetShipsInRange) _asbp_parent_spacecraft)
    (Utilities|Array|RemoveItem (Variables|Turret|GetTargetShipsInRange) _asbp_parent_spacecraft)
    (if (== _asbp_parent_spacecraft (Variables|Turret|GetCurrentTarget))
      (Variables|Turret|SetCurrentTarget 0)
      (CallFunction|FindTarget)
      (Variables|Turret|SetShootingPossible false)
      (CallFunction|ShootReleasedonServer))))

(event Custom|Shoot%20OnServer
  (bind _self self)
  ;[1 1 1] Fire Shooting
  (if (Math|Boolean|ANDBoolean (Variables|Turret|GetShootingPossible) (not (Variables|Default|GetIsBroken)) (Variables|Default|GetIsPoweredOn))
    (Utilities|FlowControl|Delay (Variables|Turret|Weapon|GetShootingDelay))
    (bind _returnvalue (Utilities|GetDataTableRow "/Game/SpaceStation/Blueprints/Weapons/Parent/DT_WeaponTypes.DT_WeaponTypes" (Variables|Turret|Weapon|GetWeaponName))
      (:then
        (if (> (Variables|Turret|Weapon|GetWeaponAmmoCurrent) 0)
          (switch Utilities|FlowControl|Switch|SwitchonE_WeaponClass (.WeaponClass (Utilities|Struct|BreakS_WeaponData _returnvalue))
            (:NewEnumerator0
              ;[1 1 1] Projectile
              (for _array_element (Components|GetChildrenComponents (Variables|Default|GetBarrels) false)
                (bind _returnvalue_2 (Game|SpawnActorfromClass (.WeaponAmmo (Utilities|Struct|BreakS_WeaponData _returnvalue)) (Math|Transform|MakeTransform (Transformation|GetWorldLocation _array_element) (Transformation|GetWorldRotation _array_element)) "AlwaysSpawn" _self _self)) ; Spawn projectile
                (bind _asbp_parent_projectile (Utilities|Casting|CastToBP_ParentProjectile _returnvalue_2))
                (Default|InitProjectile _asbp_parent_projectile (Variables|Turret|Weapon|GetWeaponName))
                ;;[1 1 1] Update Current Ammo Count
                (Variables|Turret|Weapon|SetWeaponAmmoCurrent (- (Variables|Turret|Weapon|GetWeaponAmmoCurrent) 1)))
              (CallFunction|WeapononClient))
            (:NewEnumerator1
              (if (and (Variables|Turret|GetShootingPossible) (not (Utilities|Array|IsValidIndex (Variables|Turret|Weapon|GetBeams))))
                ;[1 1 1] Beam
                (for _array_element_2 (Components|GetChildrenComponents (Variables|Default|GetBarrels) false)
                  (bind _returnvalue_3 (Game|SpawnActorfromClass (.WeaponAmmo (Utilities|Struct|BreakS_WeaponData _returnvalue)) (Math|Transform|MakeTransform (Transformation|GetWorldLocation _array_element_2) (Transformation|GetWorldRotation _array_element_2)) "AlwaysSpawn" self 0)) ; Spawn projectile
                  (bind _asbp_parent_beam (Utilities|Casting|CastToBP_ParentBeam _returnvalue_3))
                  (Default|InitBeam _asbp_parent_beam (Variables|Turret|Weapon|GetWeaponName))
                  (Transformation|AttachComponentToComponent _returnvalue_3 _array_element_2 "None" "SnapToTarget" "SnapToTarget" "SnapToTarget" true)
                  (Utilities|Array|Add (Variables|Turret|Weapon|GetBeams) _returnvalue_3))
                (CallFunction|WeapononClient)
                (bind _returnvalue_4 (Utilities|Time|SetTimerbyEvent (delegate Custom|UpdateBeamAmmoCount) (.BeamConsumptionDelay (Utilities|Struct|BreakS_WeaponData _returnvalue)) true))))))))))

(event Custom|BeginReset
  (bind _returnvalue (Utilities|Time|GetWorldDeltaSeconds))
  (bind _returnvalue_2 (Utilities|Time|GetWorldDeltaSeconds))
  (bind _platformmesh (Variables|Default|GetPlatformMesh))
  (bind _cannonmesh (Variables|Default|GetCannonMesh))
  (bind _relativerotation (Variables|/Script/Engine.SceneComponent|GetRelativeRotation _cannonmesh))
  (bind _relativerotation_2 (Variables|/Script/Engine.SceneComponent|GetRelativeRotation _platformmesh))
  (bind _returnvalue_3 (Class|KismetMathLibrary|RInterptoConstant _relativerotation "0, 0, 0" _returnvalue 5e+01))
  (bind _returnvalue_4 (Class|KismetMathLibrary|RInterptoConstant _relativerotation_2 "0, 0, 0" _returnvalue_2 5e+01))
  ;[1 1 1] Reset Aiming
  (Utilities|FlowControl|Sequence
    (:then_0
      (goto _label Open))
    (:then_1
      (Utilities|FlowControl|Gate true :!label _label
        (:Exit
          (if (not (Variables|Default|GetIsBroken))
            (Utilities|IsValid (Variables|Turret|GetCurrentTarget)
              (:Is%20Valid
                (CallFunction|CancelReset :!label _label_2))
              (:Is%20Not%20Valid
                (if (and (Math|Rotator|Equal(Rotator) _returnvalue_4 "0, 0, 0" 0.0001) (Math|Rotator|Equal(Rotator) _returnvalue_3 "0, 0, 0" 0.0001))
                  (goto _label_2)
                  (else
                    ;[1 1 1] Rotate Turret to Default Rotation
                    (Transformation|SetRelativeRotation (Variables|Default|GetPlatformMesh) _returnvalue_4 false false)
                    (Transformation|SetRelativeRotation (Variables|Default|GetCannonMesh) _returnvalue_3 false false)
                    (Utilities|FlowControl|Delay (Utilities|Time|GetWorldDeltaSeconds))
                    (CallFunction|ContinueReset)))))))))))

(event Custom|CancelAim
  (bind _turretaimingspeed (Variables|Turret|GetTurretAimingSpeed))
  ;[1 1 1] Aim At Target
  (Utilities|FlowControl|Gate true) ; enters at Close
)

(event Custom|FindTarget
  (bind _targetshipsinrange (Variables|Turret|GetTargetShipsInRange))
  ;[1 1 1] Select Target From Target Array
  (if (Utilities|Array|IsValidIndex _targetshipsinrange)
    (Variables|Turret|SetCurrentTarget (Utilities|Array|Get(acopy) _targetshipsinrange (Math|Random|RandomIntegerinRange 0 (Utilities|Array|LastIndex _targetshipsinrange))))
    (CallFunction|StartAiming)
    (else
      (CallFunction|BeginReset))))

(event Custom|StartAiming
  (bind _turretaimingspeed (Variables|Turret|GetTurretAimingSpeed))
  ;[1 1 1] Aim At Target
  (Utilities|FlowControl|Sequence
    (:then_0
      (goto _label Open))
    (:then_1
      (Utilities|FlowControl|Gate true :!label _label
        (:Exit
          (if (and (not (Variables|Default|GetIsBroken)) (Variables|Default|GetIsPoweredOn))
            (Utilities|IsValid (Variables|Turret|GetCurrentTarget)
              (:Is%20Valid
                (Variables|Turret|SetTargetLocation (Transformation|GetActorLocation (Variables|Turret|GetCurrentTarget)))
                (Variables|Turret|SetTargetAimRotator (Math|Rotator|MakeRotfromX (Math|Transform|InverseTransformDirection (Transformation|GetActorTransform) (- (Variables|Turret|GetTargetLocation) (Transformation|GetWorldLocation (Variables|Default|GetCannonMesh))))))
                ;[1 1 1] Rotate to Aim
                (Transformation|SetRelativeRotation (Variables|Default|GetPlatformMesh) (Class|KismetMathLibrary|RInterptoConstant (Variables|/Script/Engine.SceneComponent|GetRelativeRotation (Variables|Default|GetPlatformMesh)) (Math|Rotator|MakeRotator 0.0 0.0 (.Yaw (Math|Rotator|BreakRotator (Math|Rotator|MakeRotfromX (Math|Transform|InverseTransformDirection (Transformation|GetActorTransform) (- (Variables|Turret|GetTargetLocation) (Transformation|GetWorldLocation (Variables|Default|GetCannonMesh)))))))) (Utilities|Time|GetWorldDeltaSeconds) _turretaimingspeed) false false)
                (Transformation|SetRelativeRotation (Variables|Default|GetCannonMesh) (Math|Rotator|MakeRotator (.Roll (Math|Rotator|BreakRotator (Class|KismetMathLibrary|RInterptoConstant (Variables|/Script/Engine.SceneComponent|GetRelativeRotation (Variables|Default|GetCannonMesh)) (Math|Rotator|MakeRotator 0.0 (.Pitch (Math|Rotator|BreakRotator (Math|Rotator|MakeRotfromX (Math|Transform|InverseTransformDirection (Transformation|GetActorTransform) (- (Variables|Turret|GetTargetLocation) (Transformation|GetWorldLocation (Variables|Default|GetCannonMesh))))))) 0.0) (Utilities|Time|GetWorldDeltaSeconds) _turretaimingspeed))) (Math|Float|ClampAngle (.Pitch (Math|Rotator|BreakRotator (Class|KismetMathLibrary|RInterptoConstant (Variables|/Script/Engine.SceneComponent|GetRelativeRotation (Variables|Default|GetCannonMesh)) (Math|Rotator|MakeRotator 0.0 (.Pitch (Math|Rotator|BreakRotator (Math|Rotator|MakeRotfromX (Math|Transform|InverseTransformDirection (Transformation|GetActorTransform) (- (Variables|Turret|GetTargetLocation) (Transformation|GetWorldLocation (Variables|Default|GetCannonMesh))))))) 0.0) (Utilities|Time|GetWorldDeltaSeconds) _turretaimingspeed))) (Variables|Turret|GetTurretMinAngle) (Variables|Turret|GetTurretMaxAngle)) (.Yaw (Math|Rotator|BreakRotator (Class|KismetMathLibrary|RInterptoConstant (Variables|/Script/Engine.SceneComponent|GetRelativeRotation (Variables|Default|GetCannonMesh)) (Math|Rotator|MakeRotator 0.0 (.Pitch (Math|Rotator|BreakRotator (Math|Rotator|MakeRotfromX (Math|Transform|InverseTransformDirection (Transformation|GetActorTransform) (- (Variables|Turret|GetTargetLocation) (Transformation|GetWorldLocation (Variables|Default|GetCannonMesh))))))) 0.0) (Utilities|Time|GetWorldDeltaSeconds) _turretaimingspeed)))) false false)
                ;[1 1 1] Don't shoot if Ship is Already Destroyed
                (if (not (== (Variables|/Game/SpaceStation/Blueprints/SpaceCrafts/Parent/BP_ParentSpacecraft.BP_ParentSpacecraft_C|GetHullStructureCurrent (Variables|Turret|GetCurrentTarget)) 0.0))
                  (if (Math|Rotator|Equal(Rotator) (Variables|Turret|GetTargetAimRotator) (Math|Rotator|MakeRotator 0.0 (.Pitch (Math|Rotator|BreakRotator (Variables|/Script/Engine.SceneComponent|GetRelativeRotation (Variables|Default|GetCannonMesh)))) (.Yaw (Math|Rotator|BreakRotator (Variables|/Script/Engine.SceneComponent|GetRelativeRotation (Variables|Default|GetPlatformMesh))))) 1.0)
                    ;[1 1 1] Clear Sight to Shoot
                    (Utilities|FlowControl|Sequence
                      (:then_0
                        (Variables|Turret|SetShootingPossible true)
                        (CallFunction|ShootonServer))
                      (:then_1
                        (Utilities|FlowControl|Delay (Utilities|Time|GetWorldDeltaSeconds))
                        (CallFunction|ContinueAiming)))
                    (else
                      ;[1 1 1] No Clear Sight
                      (Utilities|FlowControl|Delay (Utilities|Time|GetWorldDeltaSeconds))
                      (CallFunction|ContinueAiming)
                      (Variables|Turret|SetShootingPossible false)
                      (CallFunction|ShootReleasedonServer)))))
              (:Is%20Not%20Valid
                (CallFunction|CancelAim)
                (CallFunction|BeginReset)))))))))

(event Custom|ShootReleased%20OnServer
  (bind _beams (Variables|Turret|Weapon|GetBeams))
  ;[1 1 1] Beam Off
  (Utilities|Time|PauseTimerbyHandle (stale Custom|Shoot%20OnServer _returnvalue_4))
  (for _array_element _beams
    (Utilities|IsValid _array_element
      (:Is%20Valid
        (Actor|DestroyActor _array_element))))
  (Utilities|Array|Clear _beams))

(event Custom|Weapon%20OnClient
  (bind _returnvalue (Utilities|GetDataTableRow "/Game/SpaceStation/Blueprints/Weapons/Parent/DT_WeaponTypes.DT_WeaponTypes" (Variables|Turret|Weapon|GetWeaponName))
    (:then
      ;[1 1 1] Weapon SFX
      (Audio|SpawnSoundAttached (.WeaponShootingSound (Utilities|Struct|BreakS_WeaponData _returnvalue)) (Variables|Default|GetCannonMesh) "None" "0, 0, 0" "0, 0, 0" "KeepRelativeOffset" false 1.0 (Math|Random|RandomFloatinRange 0.7 1.0) 0.0 0 0))))

(event Custom|ContinueAiming
  (bind _turretaimingspeed (Variables|Turret|GetTurretAimingSpeed))
  ;[1 1 1] Aim At Target
  (Utilities|IsValid (Variables|Turret|GetCurrentTarget)
    (:Is%20Valid
      (Utilities|FlowControl|Gate true
        (:Exit
          (if (and (not (Variables|Default|GetIsBroken)) (Variables|Default|GetIsPoweredOn))
            (Utilities|IsValid (Variables|Turret|GetCurrentTarget)
              (:Is%20Valid
                (Variables|Turret|SetTargetLocation (Transformation|GetActorLocation (Variables|Turret|GetCurrentTarget)))
                (Variables|Turret|SetTargetAimRotator (Math|Rotator|MakeRotfromX (Math|Transform|InverseTransformDirection (Transformation|GetActorTransform) (- (Variables|Turret|GetTargetLocation) (Transformation|GetWorldLocation (Variables|Default|GetCannonMesh))))))
                ;[1 1 1] Rotate to Aim
                (Transformation|SetRelativeRotation (Variables|Default|GetPlatformMesh) (Class|KismetMathLibrary|RInterptoConstant (Variables|/Script/Engine.SceneComponent|GetRelativeRotation (Variables|Default|GetPlatformMesh)) (Math|Rotator|MakeRotator 0.0 0.0 (.Yaw (Math|Rotator|BreakRotator (Math|Rotator|MakeRotfromX (Math|Transform|InverseTransformDirection (Transformation|GetActorTransform) (- (Variables|Turret|GetTargetLocation) (Transformation|GetWorldLocation (Variables|Default|GetCannonMesh)))))))) (Utilities|Time|GetWorldDeltaSeconds) _turretaimingspeed) false false)
                (Transformation|SetRelativeRotation (Variables|Default|GetCannonMesh) (Math|Rotator|MakeRotator (.Roll (Math|Rotator|BreakRotator (Class|KismetMathLibrary|RInterptoConstant (Variables|/Script/Engine.SceneComponent|GetRelativeRotation (Variables|Default|GetCannonMesh)) (Math|Rotator|MakeRotator 0.0 (.Pitch (Math|Rotator|BreakRotator (Math|Rotator|MakeRotfromX (Math|Transform|InverseTransformDirection (Transformation|GetActorTransform) (- (Variables|Turret|GetTargetLocation) (Transformation|GetWorldLocation (Variables|Default|GetCannonMesh))))))) 0.0) (Utilities|Time|GetWorldDeltaSeconds) _turretaimingspeed))) (Math|Float|ClampAngle (.Pitch (Math|Rotator|BreakRotator (Class|KismetMathLibrary|RInterptoConstant (Variables|/Script/Engine.SceneComponent|GetRelativeRotation (Variables|Default|GetCannonMesh)) (Math|Rotator|MakeRotator 0.0 (.Pitch (Math|Rotator|BreakRotator (Math|Rotator|MakeRotfromX (Math|Transform|InverseTransformDirection (Transformation|GetActorTransform) (- (Variables|Turret|GetTargetLocation) (Transformation|GetWorldLocation (Variables|Default|GetCannonMesh))))))) 0.0) (Utilities|Time|GetWorldDeltaSeconds) _turretaimingspeed))) (Variables|Turret|GetTurretMinAngle) (Variables|Turret|GetTurretMaxAngle)) (.Yaw (Math|Rotator|BreakRotator (Class|KismetMathLibrary|RInterptoConstant (Variables|/Script/Engine.SceneComponent|GetRelativeRotation (Variables|Default|GetCannonMesh)) (Math|Rotator|MakeRotator 0.0 (.Pitch (Math|Rotator|BreakRotator (Math|Rotator|MakeRotfromX (Math|Transform|InverseTransformDirection (Transformation|GetActorTransform) (- (Variables|Turret|GetTargetLocation) (Transformation|GetWorldLocation (Variables|Default|GetCannonMesh))))))) 0.0) (Utilities|Time|GetWorldDeltaSeconds) _turretaimingspeed)))) false false)
                ;[1 1 1] Don't shoot if Ship is Already Destroyed
                (if (not (== (Variables|/Game/SpaceStation/Blueprints/SpaceCrafts/Parent/BP_ParentSpacecraft.BP_ParentSpacecraft_C|GetHullStructureCurrent (Variables|Turret|GetCurrentTarget)) 0.0))
                  (if (Math|Rotator|Equal(Rotator) (Variables|Turret|GetTargetAimRotator) (Math|Rotator|MakeRotator 0.0 (.Pitch (Math|Rotator|BreakRotator (Variables|/Script/Engine.SceneComponent|GetRelativeRotation (Variables|Default|GetCannonMesh)))) (.Yaw (Math|Rotator|BreakRotator (Variables|/Script/Engine.SceneComponent|GetRelativeRotation (Variables|Default|GetPlatformMesh))))) 1.0)
                    ;[1 1 1] Clear Sight to Shoot
                    (Utilities|FlowControl|Sequence
                      (:then_0
                        (Variables|Turret|SetShootingPossible true)
                        (CallFunction|ShootonServer))
                      (:then_1
                        (Utilities|FlowControl|Delay (Utilities|Time|GetWorldDeltaSeconds))
                        (CallFunction|ContinueAiming)))
                    (else
                      ;[1 1 1] No Clear Sight
                      (Utilities|FlowControl|Delay (Utilities|Time|GetWorldDeltaSeconds))
                      (CallFunction|ContinueAiming)
                      (Variables|Turret|SetShootingPossible false)
                      (CallFunction|ShootReleasedonServer)))))
              (:Is%20Not%20Valid
                (CallFunction|CancelAim :!label _label)
                (CallFunction|BeginReset)))))))
    (:Is%20Not%20Valid
      (goto _label))))

(event Custom|ContinueReset
  (bind _returnvalue (Utilities|Time|GetWorldDeltaSeconds))
  (bind _returnvalue_2 (Utilities|Time|GetWorldDeltaSeconds))
  (bind _platformmesh (Variables|Default|GetPlatformMesh))
  (bind _cannonmesh (Variables|Default|GetCannonMesh))
  (bind _relativerotation (Variables|/Script/Engine.SceneComponent|GetRelativeRotation _cannonmesh))
  (bind _relativerotation_2 (Variables|/Script/Engine.SceneComponent|GetRelativeRotation _platformmesh))
  (bind _returnvalue_3 (Class|KismetMathLibrary|RInterptoConstant _relativerotation "0, 0, 0" _returnvalue 5e+01))
  (bind _returnvalue_4 (Class|KismetMathLibrary|RInterptoConstant _relativerotation_2 "0, 0, 0" _returnvalue_2 5e+01))
  ;[1 1 1] Reset Aiming
  (Utilities|FlowControl|Gate true
    (:Exit
      (if (not (Variables|Default|GetIsBroken))
        (Utilities|IsValid (Variables|Turret|GetCurrentTarget)
          (:Is%20Valid
            (CallFunction|CancelReset :!label _label))
          (:Is%20Not%20Valid
            (if (and (Math|Rotator|Equal(Rotator) _returnvalue_4 "0, 0, 0" 0.0001) (Math|Rotator|Equal(Rotator) _returnvalue_3 "0, 0, 0" 0.0001))
              (goto _label)
              (else
                ;[1 1 1] Rotate Turret to Default Rotation
                (Transformation|SetRelativeRotation (Variables|Default|GetPlatformMesh) _returnvalue_4 false false)
                (Transformation|SetRelativeRotation (Variables|Default|GetCannonMesh) _returnvalue_3 false false)
                (Utilities|FlowControl|Delay (Utilities|Time|GetWorldDeltaSeconds))
                (CallFunction|ContinueReset)))))))))

(event Custom|CancelReset
  (bind _returnvalue (Utilities|Time|GetWorldDeltaSeconds))
  (bind _returnvalue_2 (Utilities|Time|GetWorldDeltaSeconds))
  (bind _platformmesh (Variables|Default|GetPlatformMesh))
  (bind _cannonmesh (Variables|Default|GetCannonMesh))
  (bind _relativerotation (Variables|/Script/Engine.SceneComponent|GetRelativeRotation _cannonmesh))
  (bind _relativerotation_2 (Variables|/Script/Engine.SceneComponent|GetRelativeRotation _platformmesh))
  (bind _returnvalue_3 (Class|KismetMathLibrary|RInterptoConstant _relativerotation "0, 0, 0" _returnvalue 5e+01))
  (bind _returnvalue_4 (Class|KismetMathLibrary|RInterptoConstant _relativerotation_2 "0, 0, 0" _returnvalue_2 5e+01))
  ;[1 1 1] Reset Aiming
  (Utilities|FlowControl|Gate true) ; enters at Close
)

(event Custom|UpdateBeamAmmoCount
  (bind _currenttarget (Variables|Turret|GetCurrentTarget))
  (bind _beams (Variables|Turret|Weapon|GetBeams))
  ;[1 1 1] Beam
  (Utilities|IsValid _currenttarget
    (:Is%20Valid
      (if (Math|Boolean|ANDBoolean (not (Variables|/Game/SpaceStation/Blueprints/SpaceCrafts/Parent/BP_ParentSpacecraft.BP_ParentSpacecraft_C|GetHullBroken _currenttarget)) (Variables|Turret|GetShootingPossible) (> (Variables|Turret|Weapon|GetWeaponAmmoCurrent) 0) (not (Variables|Default|GetIsBroken)) (Variables|Default|GetIsPoweredOn))
        ;[1 1 1] Update Current Ammo Count
        (Variables|Turret|Weapon|SetWeaponAmmoCurrent (- (Variables|Turret|Weapon|GetWeaponAmmoCurrent) 1))
        (else
          ;[1 1 1] Beam Off
          (Utilities|Time|PauseTimerbyHandle (stale Custom|Shoot%20OnServer _returnvalue_4))
          (for _array_element _beams
            (Utilities|IsValid _array_element
              (:Is%20Valid
                (Actor|DestroyActor _array_element))))
          (Utilities|Array|Clear _beams))))))

(event EventBeginPlay
  ;[1 1 1] Init Targeting
  (CallFunction|FindTarget))

(fn ConstructionScript
  (|CallParentFunction)
  (Components|Sphere|SetSphereRadius (Variables|Default|GetOverlapDetection) (Variables|Turret|GetTurretSensorRadius) true))