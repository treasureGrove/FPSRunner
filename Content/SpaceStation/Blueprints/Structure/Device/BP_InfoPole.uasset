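; BP_InfoPole is a space station device that displays an advertisement while powered on, if ads are enabled.
; It extends a parent device's lifecycle, spawning the ad as a child actor component at AdLocation's transform on activation.
; The construction script also spawns the ad when the pole is unbroken, and deactivation or destruction removes the component.
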(event EventBeginPlay
  (|CallParentFunction))

(event Collision|EventActorBeginOverlap
  (params (OtherActor :type Actor%20Object%20Reference))
  (|CallParentFunction OtherActor))

(event EventTick
  (params (DeltaSeconds :type Float%20%28single-precision%29))
  (|CallParentFunction DeltaSeconds))

(event EventDeviceDestroyed
  (bind _adref (Variables|Default|GetAdRef))
  (|CallParentFunction)
  (Utilities|IsValid _adref
    (:Is%20Valid
      (Components|DestroyComponent _adref))))

(event EventActivateDevice
  (bind _adlocation (Variables|Default|GetAdLocation))
  (|CallParentFunction)
  (if (and (Variables|Control|GetShowAds) (Variables|Default|GetIsPoweredOn))
    (bind _returnvalue (AddComponent|AddChildActorComponent false (Transformation|GetRelativeTransform _adlocation)))
    (bind _output_get (Variables|Default|SetAdRef _returnvalue))
    (Transformation|SetWorldTransform _output_get (Transformation|GetWorldTransform _adlocation) false false)))

(event EventDeactivateDevice
  (bind _adref (Variables|Default|GetAdRef))
  (|CallParentFunction)
  (Utilities|IsValid _adref
    (:Is%20Valid
      (Components|DestroyComponent _adref))))

(fn ConstructionScript
  (bind _adlocation (Variables|Default|GetAdLocation))
  (|CallParentFunction)
  (if (Math|Boolean|ANDBoolean (Variables|Control|GetShowAds) (Variables|Default|GetIsPoweredOn) (not (Variables|Default|GetIsBroken)))
    (bind _returnvalue (AddComponent|AddChildActorComponent false (Transformation|GetRelativeTransform _adlocation)))
    (Variables|Default|SetAdRef _returnvalue)
    (Transformation|SetWorldTransform _returnvalue (Transformation|GetWorldTransform _adlocation) false false)))