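; Destructible meteorite item that takes weapon damage and shatters into BP_BrokenMeteorite pieces.
; Construction rolls its health from a random stream, and Hit turns on mesh physics.
; At zero health it removes its item UI and spawns offset fragments with radial impulses, more for larger scales.
; The AsteroidBroken RepNotify plays the Niagara explosion and scale-based sound, then destroys the mesh component.
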(event Custom|AsteroidExplosion%20OnServer
  (bind _returnvalue (Math|Random|RandomFloatinRange -3e+02 3e+02))
  (bind _meshworldtransform (Variables|Default|GetMeshWorldTransform))
  (bind _randomstream (Variables|Default|GetRandomStream))
  (bind _itemui_ref (Variables|Default|GetItemUI_Ref))
  (if (not (Variables|Default|GetAsteroidBroken))
    ;[1 1 1] Destroy Meteorite Mesh and UI (If existing)
    (Utilities|IsValid _itemui_ref
      (:Is%20Valid
        (Actor|DestroyActor _itemui_ref))
      (:Is%20Not%20Valid
        _))
    (Variables|Default|SetAsteroidBroken true)
    (for _index (range 0 (+ (Math|Float|Truncate (.x (Variables|Default|GetScale))) 1))
      ;[1 1 1] Spawn Broken Meteorites
      (bind _returnvalue_2 (Game|SpawnActorfromClass "/Game/SpaceStation/Blueprints/Items/BP_BrokenMeteorite.BP_BrokenMeteorite_C" (Math|Transform|MakeTransform (+ (.location _meshworldtransform) (Math|Vector|MakeVector _returnvalue _returnvalue _returnvalue)) (Class|KismetMathLibrary|RandomRotatorfromStream true (Variables|Default|GetRandomStream))) "AdjustIfPossibleButAlwaysSpawn" 0 1.0 2.0 0))
      ;[1 1 1] Add start impulse to prevent physics fighting
      (Physics|AddRadialImpulse (Variables|/Game/SpaceStation/Blueprints/Items/Parent/BP_ParentItem.BP_ParentItem_C|GetItemMesh _returnvalue_2) (Math|Vector|RotateVector (.location _meshworldtransform) (Class|KismetMathLibrary|RandomRotatorfromStream true _randomstream)) (* (.x (Variables|Default|GetScale)) 1e+01) (Math|Random|RandomFloatinRangefromStream 1e+02 1e+03 _randomstream) "RIF_Constant" true))))

(event Collision|EventHit
  (params (MyComp :type Primitive%20Component%20Object%20Reference) (Other :type Actor%20Object%20Reference) (OtherComp :type Primitive%20Component%20Object%20Reference) (bSelfMoved :type Boolean) (HitLocation :type Vector :default "0, 0, 0") (HitNormal :type Vector :default "0, 0, 0") (NormalImpulse :type Vector :default "0, 0, 0") (Hit :type Hit%20Result%20Structure%20%28by%20ref%29))
  ;[1 1 1] Set Physics when something hits (prevent issues)
  (Physics|SetSimulatePhysics (Variables|Default|GetItemMesh) true))

(event Game|Damage|EventAnyDamage
  (params (Damage :type Float%20%28single-precision%29) (DamageType :type Damage%20Type%20Object%20Reference) (InstigatedBy :type Controller%20Object%20Reference) (DamageCauser :type Actor%20Object%20Reference))
  ;[1 1 1] Recieve Weapon Damage
  (bind _output_get (Variables|Default|SetAsteroidHealth (- (Variables|Default|GetAsteroidHealth) Damage)))
  (if (and (<= _output_get 0.0) (not (Variables|Default|GetAsteroidBroken)))
    (CallFunction|AsteroidExplosiononServer)))

(event EventTick
  (params (DeltaSeconds :type Float%20%28single-precision%29))
  (|CallParentFunction DeltaSeconds) ; This node is disabled and will not be called.\nDrag off pins to build functionality.
)

(event Collision|EventActorBeginOverlap
  (params (OtherActor :type Actor%20Object%20Reference))
  (|CallParentFunction OtherActor) ; This node is disabled and will not be called.\nDrag off pins to build functionality.
)

(event EventBeginPlay
  (|CallParentFunction) ; This node is disabled and will not be called.\nDrag off pins to build functionality.
)

(fn ConstructionScript
  (|CallParentFunction)
  ;[1 1 1] Generate Random Health
  (Variables|Default|SetAsteroidHealth (Math|Random|RandomFloatinRangefromStream 1e+01 8e+01 (Variables|Default|GetRandomStream))))

(fn OnRepAsteroidBroken
  (bind _itemmesh (Variables|Default|GetItemMesh))
  ;[1 1 1] Spawn Meteorite Explosion
  (Niagara|SpawnSystemAttached "/Game/SpaceStation/Effects/Environment/NS_AsteroidExplosion.NS_AsteroidExplosion" _itemmesh "None" "0, 0, 0" "0, 0, 0" "KeepRelativeOffset" true)
  (Audio|SpawnSoundAttached (Variables|Default|GetMeteoriteExplosionSoundEffect) _itemmesh "None" "0, 0, 0" "0, 0, 0" "KeepRelativeOffset" false (Math|Float|Clamp(Float) (* (.x (Variables|Default|GetScale)) (Math|Random|RandomFloatinRangefromStream 1.0 1.5 (Variables|Default|GetRandomStream))) 0.0 2.0) 1.0 0.0 0 0)
  (Components|DestroyComponent (Variables|Default|GetItemMesh)))