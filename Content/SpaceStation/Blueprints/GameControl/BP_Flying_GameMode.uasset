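; Game mode for flying play that sets up each joining player's HUD and assigns player starts.
; On PostLogin it looks up the flying player controller's player index and passes it to that controller's ClientCreateHUD.
; The ChoosePlayerStart override returns the first PlayerStart not tagged "Used" and tags it, so each start is handed out only once, with no reset or fallback here.
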(event EventBeginPlay)

(event EventTick
  (params (DeltaSeconds :type Float%20%28single-precision%29)))

(event EventPostLogin
  (params (NewPlayer :type Player%20Controller%20Object%20Reference))
  ;[1 1 1] When Player Joins
  (bind _asbp_flying_player_controller (Utilities|Casting|CastToBP_Flying_PlayerController NewPlayer))
  (bind _playerindex (Class|TurnBasedBlueprintLibrary|GetMyPlayerIndex _asbp_flying_player_controller))
  (Default|ClientCreateHUD _asbp_flying_player_controller _playerindex NewPlayer))

(fn ConstructionScript)

(fn ChoosePlayerStart
  (params (Player :type Controller%20Object%20Reference))
  (bind _outactors (Actor|GetAllActorsOfClass "/Script/Engine.PlayerStart"))
  (for _array_element _outactors
    (if (Utilities|Name|NotEqual(Name) (Variables|/Script/Engine.PlayerStart|GetPlayerStartTag _array_element) "Used")
      (Variables|/Script/Engine.PlayerStart|SetPlayerStartTag _array_element "Used")
      (return _array_element))))