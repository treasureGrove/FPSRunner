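; Game controller that streams in the startup location with a fade-in and handles wormhole travel between space station locations.
; EnterWormhole finds the transporter matching the destination name, fades out, and swaps streamed levels.
; ExitWormhole moves the spacecraft to that transporter's exit point, taking only its yaw, then fades in.
; Only the current location's transporter stays visible and collidable, initially set by the construction script.
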(event EventBeginPlay
  (bind _returnvalue (Game|GetPlayerController 0))
  (bind _playercameramanager (Variables|/Script/Engine.PlayerController|GetPlayerCameraManager _returnvalue))
  (CameraFades|StartCameraFade :self _playercameramanager :FromAlpha 1.0 :ToAlpha 1.0 :Duration 0.1 :bShouldFadeAudio true :bHoldWhenFinished true)
  ;[1 1 1] Load First Level When Starting the Game
  (Game|LoadStreamLevel(byName) (Variables|Transportation|GetStartupLocation) true)
  (CameraFades|StartCameraFade :self _playercameramanager :FromAlpha 1.0 :Duration 2.0 :bShouldFadeAudio true :bHoldWhenFinished true))

(event Collision|EventActorBeginOverlap
  (params (OtherActor :type Actor%20Object%20Reference)))

(event EventTick
  (params (DeltaSeconds :type Float%20%28single-precision%29)))

(event Custom|EnterWormhole
  (params (DestinationLocationName :type Name) (EnteringSpacecraft :type BP%20Parent%20Spacecraft%20Object%20Reference) (Transporter :type BP%20Transporter%20Object%20Reference) (ExitingLocation :type Scene%20Component%20Object%20Reference))
  ;[1 1 1] Check if Location is Valid
  (bind _output_get (Variables|Transportation|SetDestinationLocationName DestinationLocationName))
  (Variables|Transportation|SetSpaceshipToTransport EnteringSpacecraft)
  (Variables|Transportation|SetCurrentTransporter Transporter)
  (bind (_array_element _array_index) (Utilities|Array|ForEachLoopwithBreak (Variables|Transportation|GetTransporters) :!label _label)
    (:LoopBody
      (if (Utilities|Name|Equal(Name) (Variables|/Game/SpaceStation/Blueprints/Structure/Device/BP_Transporter.BP_Transporter_C|GetCurrentLocationName _array_element) _output_get)
        (Variables|Transportation|SetLocationIsFound true)
        (Variables|Transportation|SetLocationID _array_index)
        (goto _label Break)))
    (:Completed
      (if (Variables|Transportation|GetLocationIsFound)
        ;[1 1 1] Enter Wormhole
        (CameraFades|StartCameraFade :self (Variables|/Script/Engine.PlayerController|GetPlayerCameraManager (Game|GetPlayerController 0)) :ToAlpha 1.0 :Duration 1.0 :bShouldFadeAudio true :bHoldWhenFinished true)
        (Utilities|FlowControl|Delay 1.0)
        (Game|UnloadStreamLevel(byName) (Variables|Transportation|GetCurrentLocationName) false)
        (Game|LoadStreamLevel(byName) (Variables|Transportation|GetDestinationLocationName) true)
        (Utilities|FlowControl|Delay 1.0)
        (CallFunction|ExitWormhole (Variables|Transportation|GetDestinationLocationName))
        ;[1 1 1] Hide Enter Transporter
        (Rendering|SetActorHiddenInGame (Variables|Transportation|GetCurrentTransporter) true)
        (Collision|SetActorEnableCollision (Variables|Transportation|GetCurrentTransporter) false)
        (else
          (Development|PrintString "Location not found. Make sure to have a valid DestinationLocationName!"))))))

(event Custom|ExitWormhole
  (params (CurrentLocationName :type Name))
  (bind _transporters (Variables|Transportation|GetTransporters))
  (bind _locationid (Variables|Transportation|GetLocationID))
  (bind _spaceshiptotransport (Variables|Transportation|GetSpaceshipToTransport))
  (bind _transporters_2 (Variables|Transportation|GetTransporters))
  (bind _locationid_2 (Variables|Transportation|GetLocationID))
  (bind _returnvalue (Transformation|GetActorRotation _spaceshiptotransport))
  (bind _output (Utilities|Array|Get(acopy) _transporters _locationid))
  (bind _output_2 (Utilities|Array|Get(acopy) _transporters_2 _locationid_2))
  (bind _exitingpoint (Variables|/Game/SpaceStation/Blueprints/Structure/Device/BP_Transporter.BP_Transporter_C|GetExitingPoint _output_2))
  ;[1 1 1] Exit Wormhole
  (Variables|Transportation|SetCurrentLocationName CurrentLocationName)
  (Transformation|SetActorTransform _spaceshiptotransport (Math|Transform|MakeTransform (Transformation|GetWorldLocation _exitingpoint) (Math|Rotator|MakeRotator (.roll _returnvalue) (.pitch _returnvalue) (.yaw (Transformation|GetWorldRotation _exitingpoint))) "1.000000,1.000000,1.000000"))
  (CameraFades|StartCameraFade :self (Variables|/Script/Engine.PlayerController|GetPlayerCameraManager (Game|GetPlayerController 0)) :FromAlpha 1.0 :Duration 1.0 :bShouldFadeAudio true)
  ;[1 1 1] Show Exit Transporter
  (Rendering|SetActorHiddenInGame _output false)
  (Collision|SetActorEnableCollision _output true))

(fn ConstructionScript
  (Transportation|ShowCurrentTeleporter))

(fn ShowCurrentTeleporter
  ;[1 1 1] Show only current Teleporter
  (for _array_element (Variables|Transportation|GetTransporters)
    (if (Utilities|Name|Equal(Name) (Variables|/Game/SpaceStation/Blueprints/Structure/Device/BP_Transporter.BP_Transporter_C|GetCurrentLocationName _array_element) (Variables|Transportation|GetStartupLocation))
      (Rendering|SetActorHiddenInGame _array_element false)
      (Collision|SetActorEnableCollision _array_element true)
      (else
        (Rendering|SetActorHiddenInGame _array_element true)
        (Collision|SetActorEnableCollision _array_element false)))))