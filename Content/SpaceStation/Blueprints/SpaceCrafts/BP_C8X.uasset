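; BP_C8X is a spacecraft Blueprint that builds on a parent class for its begin play, tick and construction logic.
; Its own logic keeps the two primary gun meshes visually aligned with their weapons.
; Every tick, after the parent update, it copies the relative rotation of Primary1 and Primary2 onto the matching gun meshes.
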(event Collision|EventActorBeginOverlap
  (params (OtherActor :type Actor%20Object%20Reference)))

(event EventBeginPlay
  (|CallParentFunction))

(event EventTick
  (params (DeltaSeconds :type Float%20%28single-precision%29))
  (|CallParentFunction DeltaSeconds)
  ;[1 1 1] Rotate Weapon Meshes
  (Transformation|SetRelativeRotation (Variables|Default|GetSM_Primary_Gun1) (Variables|/Script/Engine.SceneComponent|GetRelativeRotation (Variables|Default|GetPrimary1)) false false)
  (Transformation|SetRelativeRotation (Variables|Default|GetSM_Primary_Gun2) (Variables|/Script/Engine.SceneComponent|GetRelativeRotation (Variables|Default|GetPrimary2)) false false))

(fn ConstructionScript
  (|CallParentFunction))